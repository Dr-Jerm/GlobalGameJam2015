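; InteractQuest is a quest that asks the player to change the state of a randomly chosen InteractableActivate actor in the level.
; On init it picks the target, stores the opposite of its current Activated state as the goal, and shows the target's name on the quest giver's indicator widget.
; On each quest update it completes once the target's Activated state matches that goal.
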(event `self.OnQuestInit_Event`
  ;[1 1 1] Setup requirements
  (bind _outactors (`GameplayStatics.GetAllActorsOfClass` "/Game/Blueprints/InteractableActivate.InteractableActivate_C"))
  (set `self.TargetObject` (`KismetArrayLibrary.Array_Get` _outactors (`KismetMathLibrary.FFloor` (* (`KismetArrayLibrary.Array_Length` _outactors) (`KismetMathLibrary.RandomFloat`)))))
  (set `self.RequiredObjectState` (not (`/Game/Blueprints/InteractableActivate.Activated` (`self.TargetObject`))))
  ;[1 1 1] Update indicator
  (bind _asquest_indicator_widget (cast `/Game/Blueprints/QuestIndicatorWidget` (`WidgetComponent.GetUserWidgetObject` (`/Game/Blueprints/Grandmother.IndicatorWidget` (`self.QuestGiver`)))))
  (`/Game/Blueprints/QuestIndicatorWidget.SetText` _asquest_indicator_widget (`KismetStringLibrary.Concat_StrStr` "Interact with: " (`KismetSystemLibrary.GetDisplayName` (`self.TargetObject`)))))

(event `self.OnQuestUpdate_Event`
  (params (deltaTime :type "Float (single-precision)"))
  ;[1 1 1] Check if player has changed the target object's state
  (if (== (`/Game/Blueprints/InteractableActivate.Activated` (`self.TargetObject`)) (`self.RequiredObjectState`))
    (`self.Complete`)))

(fn `UserConstructionScript`
  (`parent.UserConstructionScript`))