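; BaseQuest is a base quest Blueprint that defines a timed quest lifecycle of Init, Update, Complete and Fail.
; Init resets the state flags and timer, while Complete and Fail set their flags, each firing a matching event dispatcher.
; Update accumulates elapsed time, calling Fail once it exceeds ActiveTime and otherwise broadcasting the update.
; BeginPlay binds the dispatchers to empty handler events, leaving quest-specific logic unimplemented here.
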(event `self.ReceiveBeginPlay`
  (add `self.OnQuestInit` (delegate `OnQuestInit_Event`))
  (add `self.OnQuestUpdate` (delegate `OnQuestUpdate_Event`))
  (add `self.OnQuestComplete` (delegate `OnQuestComplete_Event`))
  (add `self.OnQuestFail` (delegate `OnQuestFail_Event`)))

(event `OnQuestInit_Event`)

(event `OnQuestUpdate_Event` :!signature `self.OnQuestUpdate`
  (params (deltaTime :type "Float (double-precision)")))

(event `OnQuestComplete_Event`)

(event `OnQuestFail_Event`)

(fn `Complete`
  (set `self.IsComplete` true)
  (`self.OnQuestComplete`))

(fn `Fail`
  (`self.OnQuestFail`)
  (set `self.IsFailed` true))

(fn `Init`
  (set `self.IsComplete` false)
  (set `self.IsFailed` false)
  (set `self.ActiveTimer` 0.0)
  (`self.OnQuestInit`))

(fn `Update`
  (params (deltaTime :type "Float (double-precision)"))
  ;[1 1 1] Detect time out
  (set `self.ActiveTimer` (+ (`self.ActiveTimer`) deltaTime))
  (`/Engine/EditorBlueprintResources/StandardMacros.CompareFloat` (`self.ActiveTimer`) (`self.ActiveTime`)
    (:`>`
      (`self.Fail`))
    (:`==`
      (`self.OnQuestUpdate` deltaTime :!label _label))
    (:`<`
      (goto _label))))

(fn `UserConstructionScript`)