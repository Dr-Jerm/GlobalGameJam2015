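; Fetch quest Blueprint that tasks the player with carrying a random InteractablePickup to or away from the quest giver.
; On init it picks the target and compares its distance to FetchDistance, choosing "Bring me" if farther or "Take away" otherwise, and labels the giver's indicator.
; On update it completes once the DogeCharacter carries nothing and the target is on the required side of that distance.
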(event `self.OnQuestInit_Event`
  (bind _questgiver (`self.QuestGiver`))
  (bind _returnvalue (`KismetSystemLibrary.GetDisplayName` (`self.TargetObject`)))
  ;[1 1 1] Setup requirements
  (bind _outactors (`GameplayStatics.GetAllActorsOfClass` "/Game/Blueprints/InteractablePickup.InteractablePickup_C"))
  (set `self.TargetObject` (`KismetArrayLibrary.Array_Get` _outactors (`KismetMathLibrary.FFloor` (* (`KismetArrayLibrary.Array_Length` _outactors) (`KismetMathLibrary.RandomFloat`)))))
  (bind _returnvalue_2 (`self.GetDistanceTo` (`self.QuestGiver`) (`self.TargetObject`)))
  (`/Engine/EditorBlueprintResources/StandardMacros.CompareFloat` _returnvalue_2 (`self.FetchDistance`)
    (:`>`
      (set `self.ShouldBringTo` true))
    (:`==`
      (set `self.ShouldBringTo` false :!label _label))
    (:`<`
      (goto _label)))
  ;[1 1 1] Update indicator
  (if (`self.ShouldBringTo`)
    (`/Game/Blueprints/Grandmother.SetQuestIndicatorText` _questgiver (`KismetStringLibrary.Concat_StrStr` "Bring me: " _returnvalue))
    (else
      (`/Game/Blueprints/Grandmother.SetQuestIndicatorText` _questgiver (`KismetStringLibrary.Concat_StrStr` "Take away: " _returnvalue)))))

(event `self.OnQuestUpdate_Event`
  (params (deltaTime :type "Float (single-precision)"))
  (bind _fetchdistance (`self.FetchDistance`))
  (bind _asdoge_character (cast `/Game/Blueprints/DogeCharacter` (`GameplayStatics.GetPlayerPawn` 0)))
  (if (not (`KismetSystemLibrary.IsValid` (`/Game/Blueprints/DogeCharacter.CarryInteractive` _asdoge_character)))
    (bind _returnvalue (`self.GetDistanceTo` (`self.QuestGiver`) (`self.TargetObject`)))
    (if (`self.ShouldBringTo`)
      (`/Engine/EditorBlueprintResources/StandardMacros.CompareFloat` _returnvalue _fetchdistance
        (:`==`
          _)
        (:`<`
          _))
      (else
        (`/Engine/EditorBlueprintResources/StandardMacros.CompareFloat` _returnvalue _fetchdistance
          (:`>`
            _))))
    (`self.Complete`)))

(fn `UserConstructionScript`
  (`parent.UserConstructionScript`))