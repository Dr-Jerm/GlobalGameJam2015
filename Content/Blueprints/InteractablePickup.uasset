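; InteractablePickup is an interactable Blueprint that acts as a prototype pickup for the DogeCharacter to interact with.
; Interact calls the parent implementation, flips the PickedUp flag and prints its new value, with no attach or removal logic.
; The construction script runs the parent's script, sets a placeholder Name and assigns the static mesh from Mesh.
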(event `self.Interact`
  (params (DogeCharacter :type "/Game/Blueprints/DogeCharacter Object Reference"))
  (`parent.Interact` DogeCharacter)
  (if (`self.PickedUp`)
    (set `self.PickedUp` false)
    (else
      (set `self.PickedUp` true)))
  (`KismetSystemLibrary.PrintString` (`KismetStringLibrary.Conv_BoolToString` (`self.PickedUp`))))

(fn `UserConstructionScript`
  (`parent.UserConstructionScript`)
  (set `self.Name` "Test")
  (`StaticMeshComponent.SetStaticMesh` (`self.Mesh`)))