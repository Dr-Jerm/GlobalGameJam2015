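; Grandmother is the quest giver that assigns random quests and tracks a Love score shown on the HUD.
; Init caches the HUD widget and gathers every BaseQuest actor in the level as the quest pool.
; After an initial or between-quest delay, Tick picks and updates a quest, raising Love on completion or lowering it on failure.
; A quest indicator shows during active quests and yaws toward the player.
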(event `self.ReceiveTick`
  (params (DeltaSeconds :type "Float (single-precision)"))
  (bind _indicatorpivot (`self.IndicatorPivot`))
  ;[1 1 1] Orient quest indicator towards player
  (`SceneComponent.K2_SetWorldRotation` _indicatorpivot (`KismetMathLibrary.MakeRot` 0.0 (.yaw (`KismetMathLibrary.FindLookAtRotation` (`SceneComponent.K2_GetComponentLocation` _indicatorpivot) (`self.K2_GetActorLocation` (`GameplayStatics.GetPlayerCharacter` 0))))) false)
  ;[1 1 1] Initial Delay
  (`/Engine/EditorBlueprintResources/StandardMacros.CompareFloat` (`self.DelayTimer`) (`self.DelayTime`)
    (:`>`
      ;[1 1 1] Detect if there is a current quest
      (if (`KismetSystemLibrary.IsValid` (`self.CurrentQuest`))
        ;[1 1 1] Check if current quest is complete
        (if (`/Game/Blueprints/Quests/BaseQuest.IsComplete` (`self.CurrentQuest`))
          ;[1 1 1] Modify love value
          (set `self.Love` (+ (`self.Love`) 1))
          (`/Game/Blueprints/HUDWidget.UpdateLove` (`self.HUDWidget`) (`self.Love`) :!label _label)
          ;[1 1 1] Delay next quest
          (set `self.DelayTime` (`self.BetweenQuestDelayTime`))
          (set `self.DelayTimer` 0.0)
          (set `self.CurrentQuest` (`self.NullQuestPtr`))
          (`SceneComponent.SetVisibility` (`self.IndicatorWidget`) false false)
          (else
            ;[1 1 1] Check if current quest is failed
            (if (`/Game/Blueprints/Quests/BaseQuest.IsFailed` (`self.CurrentQuest`))
              (set `self.Love` (- (`self.Love`) 1))
              (goto _label)
              (else
                ;[1 1 1] Update Current Quest
                (`/Game/Blueprints/Quests/BaseQuest.Update` (`self.CurrentQuest`) DeltaSeconds)))))
        (else
          (`self.SelectNewQuest`))))
    (:`==`
      (set `self.DelayTimer` (+ (`self.DelayTimer`) DeltaSeconds) :!label _label_2))
    (:`<`
      (goto _label_2))))

(fn `Init`
  (params (hudWidget :type "/Game/Blueprints/HUDWidget Object Reference"))
  (set `self.HUDWidget` hudWidget)
  (bind _outactors (`GameplayStatics.GetAllActorsOfClass` "/Game/Blueprints/Quests/BaseQuest.BaseQuest_C"))
  (set `self.PossibleQuests` _outactors)
  (set `self.DelayTime` (`self.InitialDelayTime`))
  (`SceneComponent.SetVisibility` (`self.IndicatorWidget`) false false))

(fn `SelectNewQuest`
  (bind _possiblequests (`self.PossibleQuests`))
  (set `self.CurrentQuest` (`KismetArrayLibrary.Array_Get` _possiblequests (`KismetMathLibrary.FFloor` (* (`KismetArrayLibrary.Array_Length` _possiblequests) (`KismetMathLibrary.RandomFloat`)))))
  (`/Game/Blueprints/Quests/BaseQuest.Init` (`self.CurrentQuest`) self)
  (`SceneComponent.SetVisibility` (`self.IndicatorWidget`) true false))

(fn `UserConstructionScript`)